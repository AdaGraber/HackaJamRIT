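; BP_Player is the player character, handling Enhanced Input movement, camera look with invert settings, jump, crouch and sprint.
; BeginPlay adds the mapping context and creates the in-game UI and HUD; Tick writes Health to a test text display.
; Sprint goes through a server event setting IsSprinting, whose RepNotify changes walk speed; crouching while sprinting calls Slide, currently a crouch placeholder.
; Round end opens an upgrade screen populated with the supplied Boons.
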(event `self.ReceiveTick`
  (params (DeltaSeconds :type "Float (single-precision)"))
  ;[1 1 1] Testing - Health Display Text
  (`TextRenderComponent.K2_SetText` (`self.Health Text`) (`KismetTextLibrary.Conv_DoubleToText` (`self.Health`) "HalfToEven")))

(event `self.ReceiveBeginPlay`
  (bind _returnvalue (pcsubsystem `EnhancedInputLocalPlayerSubsystem` (`GameplayStatics.GetPlayerController` 0)))
  ;[0 0 0] Adds mapping context and UI (can be customized in screen), if you need to set up any variables or modifiers this would be the place
  (`/Engine/EditorBlueprintResources/StandardMacros.IsValid` _returnvalue
    (:`Is Valid`
      (`EnhancedInputSubsystemInterface.AddMappingContext` _returnvalue "/Game/EscalationContent/Inputs/Mappings/IMC_PlayerController.IMC_PlayerController" 0 (struct))
      (bind _returnvalue_2 (`|CreateWidget` "/Game/EscalationContent/Widgets/WB_inGameUI.WB_inGameUI_C"))
      (`UserWidget.AddToViewport` _returnvalue_2 0)
      (bind _returnvalue_3 (`|CreateWidget` "/Game/EscalationContent/Widgets/WB_HUD.WB_HUD_C"))
      (`UserWidget.AddToViewport` _returnvalue_3 0))))

(event `EnhancedInput|/Game/EscalationContent/Inputs/Actions/IA_LookAround`
  (params (ActionValue :type "Vector2D Structure") (ElapsedSeconds :type "Float (double-precision)") (TriggeredSeconds :type "Float (double-precision)") (InputAction :type "InputAction Object Reference" :default "/Game/EscalationContent/Inputs/Actions/IA_LookAround.IA_LookAround"))
  ;[0 0 0] Player Camera movement
  (:`Triggered`
    (`self.AddControllerYawInput` (* ActionValue_X (`KismetMathLibrary.SelectFloat` 0.0 1.0 (`self.InvertCamX`))))
    (`self.AddControllerPitchInput` (* ActionValue_Y (`KismetMathLibrary.SelectFloat` -1.0 1.0 (`self.InvertCamY`))))))

(event `EnhancedInput|/Game/EscalationContent/Inputs/Actions/IA_Jump`
  (params (ActionValue :type Boolean) (ElapsedSeconds :type "Float (double-precision)") (TriggeredSeconds :type "Float (double-precision)") (InputAction :type "InputAction Object Reference" :default "/Game/EscalationContent/Inputs/Actions/IA_Jump.IA_Jump"))
  ;[0 0 0] Jumping code
  (:`Started`
    (`self.Jump`))
  (:`Completed`
    (`self.StopJumping`)))

(event `EnhancedInput|/Game/EscalationContent/Inputs/Actions/IA_MoveAround`
  (params (ActionValue :type "Vector2D Structure") (ElapsedSeconds :type "Float (double-precision)") (TriggeredSeconds :type "Float (double-precision)") (InputAction :type "InputAction Object Reference" :default "/Game/EscalationContent/Inputs/Actions/IA_MoveAround.IA_MoveAround"))
  ;[0 0 0] Code for Movement
  (:`Triggered`
    (`self.AddMovementInput` (`self.GetActorRightVector`) ActionValue_X)
    (`self.AddMovementInput` (`self.GetActorForwardVector`) ActionValue_Y)))

(event `EnhancedInput|/Game/EscalationContent/Inputs/Actions/IA_Sprint`
  (params (ActionValue :type Boolean) (ElapsedSeconds :type "Float (double-precision)") (TriggeredSeconds :type "Float (double-precision)") (InputAction :type "InputAction Object Reference" :default "/Game/EscalationContent/Inputs/Actions/IA_Sprint.IA_Sprint"))
  ;[0 0 0] Sprinting
  (:`Triggered`
    (`self.Sprint - Server` ActionValue)))

(event `Sprint - Server`
  (params (toggleSprint :type Boolean))
  ;[0 0 0] Sprinting
  (set `self.isSprinting` toggleSprint))

(event `EnhancedInput|/Game/EscalationContent/Inputs/Actions/IA_Crouch`
  (params (ActionValue :type Boolean) (ElapsedSeconds :type "Float (double-precision)") (TriggeredSeconds :type "Float (double-precision)") (InputAction :type "InputAction Object Reference" :default "/Game/EscalationContent/Inputs/Actions/IA_Crouch.IA_Crouch"))
  ;[0 0 0] Crouch code
  (:`Started`
    (if (`self.isSprinting`)
      (`self.Slide`)
      (else
        (`self.Crouch`))))
  (:`Completed`
    (`self.UnCrouch`)))

(event `Slide`
  ;[1 0.9603 0] Starter code for sliding - TODO: Research potentially physics based sliding, temp using crouch so player does SOMETHING while not able to do slide
  (`self.Crouch`))

(event `self.OnEndRound`
  (params (Boons :type "Array of PlayerModifier Structure (by ref)"))
  ;[1 1 1] On End Round - Generate Upgrade Cards
  (`self.GenerateUpgradeCards` Boons))

(event `GenerateUpgradeCards`
  (params (Boons :type "Array of PlayerModifier Structure"))
  ;[1 1 1] On End Round - Generate Upgrade Cards
  (bind _returnvalue (`|CreateWidget` "/Game/EscalationContent/Widgets/WB_RoundEnd.WB_RoundEnd_C"))
  (`UserWidget.AddToViewport` _returnvalue 0)
  (`/Game/EscalationContent/Widgets/WB_RoundEnd.SetBoons` _returnvalue Boons))

(fn `OnRep_isSprinting`
  (set `CharacterMovementComponent.MaxWalkSpeed` (`KismetMathLibrary.SelectFloat` 600.0 300.0 (`self.isSprinting`)) (`self.CharacterMovement`)))

(fn `UserConstructionScript`)